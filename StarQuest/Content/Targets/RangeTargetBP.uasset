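; RangeTargetBP is a shooting-range target that slides back and forth and awards points when shot.
; On BeginPlay it caches the player character, then two chained timelines ping-pong it between its start location and a hard-coded Y position.
; Head and Body overlaps with BP_Bullet add to the character's Points, more for the head, and play a metal hit sound.
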(event OnComponentBeginOverlap(Head)
  (params (OverlappedComponent :type Primitive%20Component%20Object%20Reference) (OtherActor :type Actor%20Object%20Reference) (OtherComp :type Primitive%20Component%20Object%20Reference) (OtherBodyIndex :type Integer) (bFromSweep :type Boolean) (SweepResult :type Hit%20Result%20Structure%20%28by%20ref%29))
  (bind _charref (Variables|Default|GetCharRef))
  (Utilities|Casting|CastToBP_Bullet OtherActor)
  (Variables|/Game/AnimStarterPack/Ue4ASP_Character.Ue4ASP_Character_C|SetPoints _charref (+ (Variables|/Game/AnimStarterPack/Ue4ASP_Character.Ue4ASP_Character_C|GetPoints _charref) 5))
  (Audio|PlaySoundatLocation "/Game/Sound/Gunhit_Metal.Gunhit_Metal" (Transformation|GetActorLocation) "0, 0, 0" 0.5 1.0 0.0 0 0 0))

(event OnComponentBeginOverlap(Body)
  (params (OverlappedComponent :type Primitive%20Component%20Object%20Reference) (OtherActor :type Actor%20Object%20Reference) (OtherComp :type Primitive%20Component%20Object%20Reference) (OtherBodyIndex :type Integer) (bFromSweep :type Boolean) (SweepResult :type Hit%20Result%20Structure%20%28by%20ref%29))
  (bind _charref (Variables|Default|GetCharRef))
  (Utilities|Casting|CastToBP_Bullet OtherActor)
  (Variables|/Game/AnimStarterPack/Ue4ASP_Character.Ue4ASP_Character_C|SetPoints _charref (+ (Variables|/Game/AnimStarterPack/Ue4ASP_Character.Ue4ASP_Character_C|GetPoints _charref) 1))
  (Audio|PlaySoundatLocation "/Game/Sound/Gunhit_Metal.Gunhit_Metal" (Transformation|GetActorLocation) "0, 0, 0" 0.5 1.0 0.0 0 0 0))

(event EventBeginPlay
  (bind _returnvalue (Transformation|GetActorLocation))
  (Variables|Default|SetStart (Math|Vector|MakeVector (.x _returnvalue) (.y _returnvalue) (.z _returnvalue)))
  (Variables|Default|Setend (Math|Vector|MakeVector (.x _returnvalue) 845.0 (.z _returnvalue)))
  (bind _asue_4asp_character (Utilities|Casting|CastToUe4ASP_Character (Game|GetPlayerCharacter 0)))
  (Variables|Default|SetCharRef _asue_4asp_character)
  (bind _move (Timeline|Move Play)
    (:Update
      (Transformation|SetActorRelativeLocation (Math|Vector|Lerp(Vector) (Variables|Default|GetStart) (Variables|Default|Getend) _move)))
    (:Finished
      (bind _move_2 (Timeline|Move2 ReverseFromEnd)
        (:Update
          (Transformation|SetActorRelativeLocation (Math|Vector|Lerp(Vector) (Variables|Default|GetStart) (Variables|Default|Getend) _move_2)))
        (:Finished
          (Timeline|Move PlayFromStart))))))

(fn ConstructionScript)