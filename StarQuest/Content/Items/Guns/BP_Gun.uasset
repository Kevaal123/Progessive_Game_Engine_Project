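; BP_Gun is an interactable gun that players can pick up, drop and fire.
; A Dropped/Equipped state toggles mesh physics and the collision profiles of the sphere and mesh, starting Dropped on BeginPlay.
; Interacting passes the gun to the player's PickUpGun, then equips it.
; Fire spawns a BP_Bullet at the barrel socket, aimed at a distant point along the camera's forward vector without tracing.
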(event EventBeginPlay
  (Private|SetGunState "NewEnumerator0"))

(event EventOnInteracted
  (params (Player :type Ue%204ASP%20Character%20Object%20Reference))
  (Default|PickUpGun Player self)
  (Private|SetGunState "NewEnumerator1"))

(fn ConstructionScript
  (|CallParentFunction))

(fn GetInteractionText
  (return "Pick Up"))

(fn GetInteractionTextAttached
  (return (Variables|Default|GetSkeletalMesh)))

(fn SetGunState
  (params (NewGun%20State :type EGunState%20Enum :default "NewEnumerator0"))
  (bind _skeletalmesh (Variables|Default|GetSkeletalMesh))
  (bind _skeletalmesh_2 (Variables|Default|GetSkeletalMesh))
  (bind _output_get (Variables|Private|SetGun%20State NewGun%20State))
  (switch Utilities|FlowControl|Switch|SwitchonEGunState _output_get
    (:NewEnumerator0
      (Collision|SetCollisionProfileName (Variables|Default|GetSphere) "OverlapAllDynamic" true :!class /Script/Engine.PrimitiveComponent)
      (Physics|SetSimulatePhysics _skeletalmesh true)
      (Collision|SetCollisionProfileName _skeletalmesh "DroppedGun" true :!class /Script/Engine.PrimitiveComponent))
    (:NewEnumerator1
      (Collision|SetCollisionProfileName (Variables|Default|GetSphere) "NoCollision" true :!class /Script/Engine.PrimitiveComponent)
      (Physics|SetSimulatePhysics _skeletalmesh_2 false)
      (Collision|SetCollisionProfileName _skeletalmesh_2 "NoCollision" true :!class /Script/Engine.PrimitiveComponent)
      (Transformation|ResetRelativeTransform (Variables|Default|GetSkeletalMesh)))))

(fn Drop
  (Private|SetGunState "NewEnumerator0"))

(fn Fire
  (params (PlayerCamera :type Camera%20Component%20Object%20Reference))
  (bind _skeletalmesh (Variables|Default|GetSkeletalMesh))
  (bind _returnvalue (Transformation|GetSocketLocation _skeletalmesh "Bullet_Barrel"))
  (Game|SpawnActorfromClass "/Game/Items/Bullet/BP_Bullet.BP_Bullet_C" (Math|Transform|MakeTransform _returnvalue "0, 0, 0" "1,1,1") "Undefined" 0 (* (Math|Vector|Normalize (- (+ (Transformation|GetWorldLocation PlayerCamera) (* (Math|Vector|GetForwardVector PlayerCamera) 1e+04)) _returnvalue)) 1e+04) 0))